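; BP_BallPlayer is the player ball in the RollingBall game, moved by applying physics force to its Sphere component.
; On BeginPlay it adds the IM_Controls mapping context to player 0's Enhanced Input subsystem.
; While IA_Control triggers, it swaps the 2D input axes into a horizontal world-space vector, scales it by Speed and applies it as a mass-independent acceleration.
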(event Input|EnhancedActionEvents|EnhancedInputActionIA_Control
  (params (ActionValue :type Vector%202D%20Structure) (ElapsedSeconds :type Float%20%28double-precision%29) (TriggeredSeconds :type Float%20%28double-precision%29) (InputAction :type Input%20Action%20Object%20Reference :default "/Game/RollingBall/Input/Action/IA_Control.IA_Control"))
  (bind (_x _y) (Math|Vector2D|BreakVector2D ActionValue))
  ;[1 1 1] Sphereに力を加える
  (:Triggered
    (Physics|AddForce (Variables|Default|GetSphere) (* (Math|Vector|MakeVector _y _x 0.0) (Variables|Default|GetSpeed)) "None" true)))

(event EventBeginPlay
  (bind _returnvalue (Game|GetPlayerController 0))
  (bind _returnvalue_2 (PlayerController|LocalPlayerSubsystems|GetEnhancedInputLocalPlayerSubsystem _returnvalue))
  ;[1 1 1] Input方法をIM_Controlい設定する
  (Utilities|IsValid _returnvalue_2
    (:Is%20Valid
      (Input|AddMappingContext _returnvalue_2 "/Game/RollingBall/Input/IM_Controls.IM_Controls" 0 "(bIgnoreAllPressedKeysUntilRelease=True,bForceImmediately=False,bNotifyUserSettings=False)"))))

(event Collision|EventActorBeginOverlap
  (params (OtherActor :type Actor%20Object%20Reference)))

(event EventTick
  (params (DeltaSeconds :type Float%20%28single-precision%29)))

(fn ConstructionScript)